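; Elevator button Blueprint that calls its referenced Elevator to move or signals that the call is rejected.
; CallElevator moves the Elevator only when the button's UpOrDown value matches the Elevator's own.
; On a mismatch, CheckLight flashes red and returns to green after a short delay.
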(event Custom|CallElevator
  (if (== (Variables|Default|GetUpOrDown) (Variables|/Game/Blueprints/Elevator.Elevator_C|GetUpOrDown (Variables|Default|GetElevator)))
    (Default|MoveElevator (Variables|Default|GetElevator))
    (else
      (Rendering|Components|Light|SetLightColor (Variables|Default|GetCheckLight) "(R=0.439657,G=0.000000,B=0.000000,A=1.000000)" true)
      (Utilities|FlowControl|Delay 0.3)
      (Rendering|Components|Light|SetLightColor (Variables|Default|GetCheckLight) "(R=0.013702,G=0.445201,B=0.000000,A=1.000000)" true))))

(fn ConstructionScript)