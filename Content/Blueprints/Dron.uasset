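; Drone enemy that patrols a spline path and shoots at a character it can see within its detection sphere.
; A looping timeline, driven from Tick, moves and rotates the Cone along the spline, pausing during combat.
; Sphere overlaps set the target, and an object line trace from the Arrow confirms sight, counting a Gun hit as visible.
; While visible, the drone faces the character and spawns shots on a delayed re-check loop.
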(event OnComponentBeginOverlap(Sphere)
  (params (OverlappedComponent :type Primitive%20Component%20Object%20Reference) (OtherActor :type Actor%20Object%20Reference) (OtherComp :type Primitive%20Component%20Object%20Reference) (OtherBodyIndex :type Integer) (bFromSweep :type Boolean) (SweepResult :type Hit%20Result%20Structure%20%28by%20ref%29))
  ;[1 1 1] Проверка пересёкся ли дрон с персонажем. Если да, активируем флаг проверки видимости
  (bind _ascharacter (Utilities|Casting|CastToCharacter OtherActor))
  (Variables|Default|SetCharacter _ascharacter)
  (Variables|Default|SetRightTarget true))

(event OnComponentEndOverlap(Sphere)
  (params (OverlappedComponent :type Primitive%20Component%20Object%20Reference) (OtherActor :type Actor%20Object%20Reference) (OtherComp :type Primitive%20Component%20Object%20Reference) (OtherBodyIndex :type Integer))
  ;[1 1 1] Проверка вышел ли персонаж из зоны действия дрона. Если да то отключаем бой и флаг проверки видимости.
  (Utilities|Casting|CastToCharacter OtherActor)
  (Variables|Default|SetRightTarget false)
  (Variables|Default|SetCharacter 0)
  (Variables|Default|SetFight false))

(event Custom|MoveDron
  ;[1 1 1] Движение дрона
  ;[1 1 1] Проверка на продолжение движения дрона
  (if (Variables|Default|GetRepeat)
    (Variables|Default|SetRepeat false)
    (bind _moving_drone (Timeline|Moving PlayFromStart)
      (:Update
        ;[1 1 1] Движение дрона по траектории
        (Transformation|SetWorldLocation (Variables|Default|GetCone) (Spline|GetLocationatTime (Variables|Default|GetSpline) _moving_drone "World" false) false false)
        ;[1 1 1] Поворот дрона во время движения
        (Transformation|SetWorldRotation (Variables|Default|GetCone) (Math|Rotator|MakeRotator (.Roll (Math|Rotator|BreakRotator (Class|SplineComponent|GetRotationatTime (Variables|Default|GetSpline) _moving_drone "World" false))) -9e+01 (.Yaw (Math|Rotator|BreakRotator (Class|SplineComponent|GetRotationatTime (Variables|Default|GetSpline) _moving_drone "World" false)))) false false))
      (:Finished
        (Variables|Default|SetRepeat true)))
    (else
      ;[1 1 1] Проверка находится ли дрон в бою
      (if (Variables|Default|GetFight)
        (Timeline|Moving Stop)
        (else
          (Timeline|Moving Play))))))

(event Custom|StartFight
  (bind _character (Variables|Default|GetCharacter))
  (bind _cone (Variables|Default|GetCone))
  (bind _returnvalue (Transformation|GetWorldLocation _cone))
  (bind _capsulecomponent (Variables|/Script/Engine.Character|GetCapsuleComponent _character))
  (bind _returnvalue_2 (Components|GetChildComponent _capsulecomponent 4))
  (bind _returnvalue_3 (Transformation|GetWorldLocation _returnvalue_2))
  (bind _returnvalue_4 (Math|Rotator|FindLookatRotation _returnvalue _returnvalue_3))
  (bind (_roll _pitch _yaw) (Math|Rotator|BreakRotator _returnvalue_4))
  ;[1 1 1] Режим атаки
  ;[1 1 1] Разворот дрона в направлении персонажа
  (Transformation|SetWorldRotation (Variables|Default|GetCone) (Math|Rotator|MakeRotator _roll -9e+01 _yaw) false false)
  ;[1 1 1] Стрельба
  (Game|SpawnActorfromClass "/Game/Weapon/MissileOrigin.MissileOrigin_C" (Transformation|GetWorldTransform (Variables|Default|GetArrow)) "AlwaysSpawn" 0 0))

(event Custom|CheckTarget
  ;[1 1 1] Проверка видимости
  ;[1 1 1] Если персонаж в зоне действия дрона выпускаем в него луч
  (if (Variables|Default|GetRightTarget)
    (bind _outhit (Collision|LineTraceForObjects (Transformation|GetWorldLocation (Variables|Default|GetArrow)) (Transformation|GetWorldLocation (Components|GetChildComponent (Variables|/Script/Engine.Character|GetCapsuleComponent (Variables|Default|GetCharacter)) 4)) (Utilities|Array|MakeArray "ObjectTypeQuery1" "ObjectTypeQuery2") false 0 "ForOneFrame"))
    ;[1 1 1] Если луч уперается в персонажа, то активируем флаг атаки. Если между персонажем и дроном укрытие, то флаг становится не активным.
    (Utilities|Casting|CastToCharacter (.HitActor (Collision|BreakHitResult _outhit))
      (:then
        (Variables|Default|SetFight true :!label _label))
      (:CastFailed
        (Utilities|Casting|CastToGun (.HitActor (Collision|BreakHitResult _outhit))
          (:then
            (goto _label))
          (:CastFailed
            (Variables|Default|SetFight false)))))))

(event EventTick
  (params (DeltaSeconds :type Float%20%28single-precision%29))
  (CallFunction|MoveDron)
  (if (not (Variables|Default|GetFight))
    (CallFunction|CheckTarget :!label _label)
    (if (Variables|Default|GetFight)
      (CallFunction|StartFight)
      (Utilities|FlowControl|Delay 0.4)
      (goto _label))))

(fn ConstructionScript)