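; Door actor that swings a static mesh open and closed by yawing it between 0 and 90 degrees.
; OpenCloseDoor picks OpenDoor or CloseDoor from OpenFlag.
; Each event animates by calling itself after a short Delay, stepping Rotate without a Timeline.
; OpenFlag and the Name label update only when Rotate exactly hits the end angle, with no guard for calls mid-swing.
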(event Custom|CloseDoor
  (Transformation|SetRelativeRotation (Variables|Default|GetSM_Door) (Math|Rotator|MakeRotator 0.0 0.0 (Variables|Default|GetRotate)) false false)
  (Utilities|FlowControl|Delay 0.01)
  (Variables|Default|SetRotate (- (Variables|Default|GetRotate) 2.0))
  (if (== (Variables|Default|GetRotate) 0.0)
    (Variables|Default|SetName (Utilities|String|StringToName (Variables|Default|GetNameOpenDoor)))
    (Variables|Default|SetOpenFlag false)
    (else
      (CallFunction|CloseDoor))))

(event Custom|OpenDoor
  (Transformation|SetRelativeRotation (Variables|Default|GetSM_Door) (Math|Rotator|MakeRotator 0.0 0.0 (Variables|Default|GetRotate)) false false)
  (Utilities|FlowControl|Delay 0.01)
  (Variables|Default|SetRotate (+ (Variables|Default|GetRotate) 2.0))
  (if (== (Variables|Default|GetRotate) 9e+01)
    (Variables|Default|SetName (Utilities|String|StringToName (Variables|Default|GetNameCloseDoor)))
    (Variables|Default|SetOpenFlag true)
    (else
      (CallFunction|OpenDoor))))

(fn ConstructionScript)

(fn OpenCloseDoor
  (if (Variables|Default|GetOpenFlag)
    (CallFunction|CloseDoor)
    (else
      (CallFunction|OpenDoor))))