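; BaseLamp is a lamp Blueprint whose point light flickers off briefly at random intervals.
; From BeginPlay, SwitchLight sets the intensity high, holds it for a random delay of several seconds, then drops it to zero for a moment.
; The Repeat event wires back to the start, forming an endless Delay-driven loop without Tick or timers.
; The construction script and OnRep_ReturnFlashCount are empty.
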(event Custom|Repeat
  (CallFunction|SwitchLight 1e+04)
  (Utilities|FlowControl|Delay (Math|Random|RandomFloatinRange 4.0 15.0))
  (CallFunction|SwitchLight 0.0)
  (Utilities|FlowControl|Delay 0.1)
  (CallFunction|Repeat))

(event EventBeginPlay
  (CallFunction|SwitchLight 1e+04)
  (Utilities|FlowControl|Delay (Math|Random|RandomFloatinRange 4.0 15.0))
  (CallFunction|SwitchLight 0.0)
  (Utilities|FlowControl|Delay 0.1)
  (CallFunction|Repeat))

(fn ConstructionScript)

(fn SwitchLight
  (params (Intensity :type Float%20%28double-precision%29))
  (Rendering|Components|Light|SetIntensity (Variables|Default|GetPointLight) Intensity)
  (return))

(fn OnRepReturnFlashCount)